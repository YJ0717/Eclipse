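; Player Blueprint that manages the player's UI and a few trait and skill variables.
; BeginPlay adds the User_HUD widget and runs the stat fps console command.
; B shows the cursor and opens Trait_Select, while PlayerDieUI shows the YouDie widget for a few seconds.
; G flip-flops SkillAttack between two values, and the Shufle event shuffles the AllTraits array in place.
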(event Custom|Shufle
  (bind _output_get (Variables|Default|SetAllTraits (Variables|Default|GetAllTraits)))
  (Utilities|Array|Shuffle _output_get))

(event EventBeginPlay
  ;[0.15 0.15 0.15 0.5] UI
  (Development|ExecuteConsoleCommand "stat fps" 0)
  (bind _returnvalue (UserInterface|CreateWidget "/Game/UI/User_HUD.User_HUD_C" (Game|GetPlayerController 0)))
  (bind _output_get (Variables|Default|SetNewVar _returnvalue))
  (UserInterface|Viewport|AddtoViewport _output_get 0))

(event Collision|EventActorBeginOverlap
  (params (OtherActor :type Actor%20Object%20Reference)))

(event EventTick
  (params (DeltaSeconds :type Float%20%28single-precision%29)))

(event EventPlayerDieUI
  (bind _returnvalue (UserInterface|CreateWidget "/Game/UI/YouDie.YouDie_C"))
  (bind _output_get (Variables|Default|SetNewVar_2 _returnvalue))
  (UserInterface|Viewport|AddtoViewport _output_get 0)
  (Utilities|FlowControl|Delay 5.0)
  (Widget|RemovefromParent _output_get))

(event Input|KeyboardEvents|B
  (params (Key :type Key%20Structure :default "None"))
  ;[0.15 0.15 0.15 0.5] Setting
  (:Pressed
    (Variables|/Script/Engine.PlayerController|SetbShowMouseCursor (Game|GetPlayerController 0) true)
    (bind _returnvalue (UserInterface|CreateWidget "/Game/UI/Trait_Select.Trait_Select_C"))
    (bind _output_get (Variables|Default|SetNewVar_1 _returnvalue))
    (UserInterface|Viewport|AddtoViewport _output_get 0)))

(event Input|KeyboardEvents|G
  (params (Key :type Key%20Structure :default "None"))
  (:Pressed
    (Utilities|FlowControl|FlipFlop
      (:A
        (Variables|Default|SetSkillAttack 2.0))
      (:B
        (Variables|Default|SetSkillAttack 1.0)))))

(fn ConstructionScript)