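; BP_Sg4BossCharacter is the Stage 4 boss character Blueprint, handling the boss's health bar and victory UI.
; BeginPlay adds a Boss4_HPUI1 widget to the viewport, and Tick refreshes its HPBar from CurrentHealth over MaxHealth every frame.
; The DieUI event shows the Victory widget, then removes it after a five-second delay.
; The graph contains no combat, damage or death logic and no call to DieUI.
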(event EventBeginPlay
  (bind _returnvalue (UserInterface|CreateWidget "/Game/UI/Boss4_HPUI1.Boss4_HPUI1_C"))
  (bind _output_get (Variables|Default|SetNewVar _returnvalue))
  (UserInterface|Viewport|AddtoViewport _output_get 0))

(event Collision|EventActorBeginOverlap
  (params (OtherActor :type Actor%20Object%20Reference)))

(event EventTick
  (params (DeltaSeconds :type Float%20%28single-precision%29))
  (Progress|SetPercent (Variables|/Game/UI/Boss4_HPUI1.Boss4_HPUI1_C|GetHPBar (Variables|Default|GetNewVar)) (/ (Variables|Default|GetCurrentHealth) (Variables|Default|GetMaxHealth))))

(event EventDieUI
  (bind _returnvalue (UserInterface|CreateWidget "/Game/UI/Victory.Victory_C"))
  (bind _output_get (Variables|Default|SetNewVar_0 _returnvalue))
  (UserInterface|Viewport|AddtoViewport _output_get 0)
  (Utilities|FlowControl|Delay 5.0)
  (Widget|RemovefromParent _output_get))

(fn ConstructionScript)