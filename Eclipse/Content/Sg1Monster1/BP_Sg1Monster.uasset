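; BP_Sg1Monster is a monster Blueprint that shows blood effects when hurt and displays a health bar.
; OnDamagedBP spawns a Niagara blood system at the actor's location.
; Tick casts the widget component's widget to Monster1_HPUI1 and sets its HP bar to the ratio of Health to MaxHealth every frame.
; BeginPlay also creates a Monster1_HPUI1 widget, but the graph does not use it.
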(event EventBeginPlay
  (UserInterface|CreateWidget "/Game/UI/Monster1_HPUI1.Monster1_HPUI1_C" 0 0))

(event Collision|EventActorBeginOverlap
  (params (OtherActor :type Actor%20Object%20Reference)))

(event EventTick
  (params (DeltaSeconds :type Float%20%28single-precision%29))
  (bind _asmonster_1_hpui1 (Utilities|Casting|CastToMonster1_HPUI1 (UserInterface|GetWidget (Variables|Default|GetWidget))))
  (Progress|SetPercent (Variables|/Game/UI/Monster1_HPUI1.Monster1_HPUI1_C|GetHPBar _asmonster_1_hpui1) (/ (Variables|Default|GetHealth) (Variables|Default|GetMaxHealth))))

(event EventOnDamagedBP
  (Niagara|SpawnSystematLocation "/Game/DH_VFX/Blood/Blood.Blood" (Transformation|GetActorLocation)))

(fn ConstructionScript)