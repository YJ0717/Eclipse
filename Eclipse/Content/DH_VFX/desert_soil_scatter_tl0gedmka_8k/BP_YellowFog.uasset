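; BP_YellowFog is an actor, apparently a yellow fog or storm effect judging by its names, that trails the player.
; Each Tick, while it is more than a fixed distance from player character 0, it moves toward that character by StormSpeed along the unit direction.
; The move has no sweep and is not scaled by delta time, so its speed depends on frame rate.
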(event EventBeginPlay)

(event Collision|EventActorBeginOverlap
  (params (OtherActor :type Actor%20Object%20Reference)))

(event EventTick
  (params (DeltaSeconds :type Float%20%28single-precision%29))
  (bind _returnvalue (Game|GetPlayerCharacter 0))
  (bind _returnvalue_2 (Transformation|GetActorLocation))
  (bind _returnvalue_3 (Transformation|GetActorLocation _returnvalue))
  (if (> (Math|Vector|Distance(Vector) _returnvalue_2 _returnvalue_3) 5e+03)
    (Transformation|SetActorLocation (+ (Transformation|GetActorLocation) (* (Math|Vector|GetUnitDirection(Vector) _returnvalue_2 _returnvalue_3) (Variables|Default|GetStormSpeed))) false false)))

(fn ConstructionScript)