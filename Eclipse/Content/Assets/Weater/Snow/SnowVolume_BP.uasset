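; Snow weather volume that drives box-sized Niagara snowfall, snow and wind-scaled blizzard audio, material snow buildup and height fog density.
; The construction script pushes spawn range, amount, size, colour, wind and gravity to Niagara, while Tick keeps world rotation at zero.
; SetSnowAmount fades particles and volume via timelines, then restarts a looping timer that accumulates or melts snow, updates fog and stops itself at the limits.
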(event Custom|AdjustSnow
  (bind _snowamount (Variables|Spawn|GetSnowAmount))
  ;[0 0 0] Based on amount of rain, either increase or decrease the wetness amount. Clamped between 0 and 4 as per the material settings.
  (if (< _snowamount 1e+02)
    (bind _returnvalue (Rendering|Material|GetScalarParameterValue 0 "SnowAmount" :!class /Script/Engine.KismetMaterialLibrary))
    (Rendering|Material|SetScalarParameterValue 0 "SnowAmount" (- _returnvalue (Math|Float|MapRangeClamped _snowamount 0.0 1e+02 0.0006 0.0001)) :!class /Script/Engine.KismetMaterialLibrary)
    (else
      (bind _returnvalue_2 (Rendering|Material|GetScalarParameterValue 0 "SnowAmount" :!class /Script/Engine.KismetMaterialLibrary))
      (Rendering|Material|SetScalarParameterValue 0 "SnowAmount" (+ _returnvalue_2 (Math|Float|MapRangeClamped _snowamount 1e+03 1e+04 5e-05 0.0006)) :!class /Script/Engine.KismetMaterialLibrary)))
  (bind _returnvalue_3 (Rendering|Material|GetScalarParameterValue 0 "SnowAmount" :!class /Script/Engine.KismetMaterialLibrary))
  (bind _returnvalue_4 (Actor|GetActorOfClass "/Script/Engine.ExponentialHeightFog"))
  (Class|ExponentialHeightFogComponent|SetFogDensity (Variables|/Script/Engine.ExponentialHeightFog|GetComponent _returnvalue_4) (Math|Float|MapRangeClamped _returnvalue_3 0.0 4.0 0.0436 3.0))
  (if (or (<= _returnvalue_3 0.0) (>= _returnvalue_3 4.0))
    (Utilities|FlowControl|Delay 0.2)
    (Utilities|Time|ClearTimerbyFunctionName 0 "AdjustSnow")))

(event Custom|SetSnowAmount
  (params (Amount :type Float%20%28double-precision%29))
  ;[0 0 0] Set rain amount by adjusting spawn amount in niagara and set volume accordingly.
  (Variables|Default|SetCurrentVolume (Variables|/Script/Engine.AudioComponent|GetVolumeMultiplier (Variables|Default|GetSnow_Audio)))
  (Utilities|FlowControl|Sequence
    (:then_0
      (bind _value (Timeline|SetSnow PlayFromStart)
        (:Update
          (Niagara|SetNiagaraVariable(Float) (Variables|Default|GetSnow_NS) "SnowAmount" (Math|Float|Lerp (Variables|Spawn|GetSnowAmount) Amount _value)))
        (:Finished
          (Variables|Spawn|SetSnowAmount Amount)
          (bind _returnvalue (Rendering|Material|GetScalarParameterValue 0 "SnowAmount" :!class /Script/Engine.KismetMaterialLibrary))
          (if (<= _returnvalue 0.0)
            (Rendering|Material|SetScalarParameterValue 0 "SnowAmount" 0.01 :!class /Script/Engine.KismetMaterialLibrary)
            (elif (>= _returnvalue 4.0)
              (Rendering|Material|SetScalarParameterValue 0 "SnowAmount" 3.99 :!class /Script/Engine.KismetMaterialLibrary)))
          (Utilities|Time|SetTimerbyFunctionName 0 "AdjustSnow" 0.01 true))))
    (:then_1
      (Utilities|FlowControl|RetriggerableDelay 1.0)
      (bind _value_2 (Timeline|SetSnowVolume PlayFromStart)
        (:Update
          (Audio|Components|Audio|SetVolumeMultiplier (Variables|Default|GetSnow_Audio) (Math|Float|Lerp (Variables|Default|GetCurrentVolume) (CallFunction|GetBlizzardAudio Amount) _value_2) :!class /Script/Engine.AudioComponent))))))

(event EventTick
  (params (DeltaSeconds :type Float%20%28single-precision%29))
  ;[0 0 0] Zero out rotation when attached to actor.
  (Transformation|SetActorRotation "0, 0, 0"))

(event EventBeginPlay
  ;[0 0 0] Increase/decrease wetness amount using timer.
  (Utilities|Time|SetTimerbyFunctionName 0 "AdjustSnow" 0.01 true)
  (Audio|Components|Audio|SetVolumeMultiplier (Variables|Default|GetSnow_Audio) (CallFunction|GetBlizzardAudio (Variables|Spawn|GetSnowAmount)) :!class /Script/Engine.AudioComponent))

(fn ConstructionScript
  (bind _spawnrange (Variables|Spawn|GetSpawnRange))
  (bind _snow_ns (Variables|Default|GetSnow_NS))
  (bind _colour (Variables|Look|GetColour))
  ;[1 1 1] Set rain settings.
  (Components|Box|SetBoxExtent (Variables|Default|GetSpawnBox) _spawnrange true)
  (Niagara|SetNiagaraVariable(Vector3) _snow_ns "SpawnRange" _spawnrange)
  (Niagara|SetNiagaraVariable(Float) _snow_ns "SnowAmount" (Variables|Spawn|GetSnowAmount))
  (Niagara|SetNiagaraVariable(Float) _snow_ns "SizeMultiplier" (Variables|Spawn|GetSize))
  (Niagara|SetNiagaraVariable(LinearColor) _snow_ns "SnowColour" (Utilities|Struct|MakeLinearColor (.r _colour) (.g _colour) (.b _colour) (Variables|Look|GetOpacity)))
  (Niagara|SetNiagaraVariable(Vector3) _snow_ns "WindMin" (Math|Vector|MakeVector (.x (Variables|Velocity|GetWindX)) (.x (Variables|Velocity|GetWindY)) (.x (Variables|Velocity|GetGravity))))
  (Niagara|SetNiagaraVariable(Vector3) _snow_ns "WindMax" (Math|Vector|MakeVector (.y (Variables|Velocity|GetWindX)) (.y (Variables|Velocity|GetWindY)) (.y (Variables|Velocity|GetGravity)))))

(fn GetBlizzardAudio
  (params (SnowAmount :type Float%20%28double-precision%29))
  (bind _windx (Variables|Velocity|GetWindX))
  (bind _windy (Variables|Velocity|GetWindY))
  (bind _returnvalue (Math|Float|Absolute(Float) (.y _windy)))
  (bind _returnvalue_2 (Math|Float|Absolute(Float) (.x _windy)))
  (bind _returnvalue_3 (Math|Float|Absolute(Float) (.x _windx)))
  (bind _returnvalue_4 (Math|Float|Absolute(Float) (.y _windx)))
  (bind _returnvalue_5 (Math|Float|MapRangeClamped SnowAmount 0.0 2e+04 0.0 1.0))
  (bind _returnvalue_6 (Math|Float|Max(Float) _returnvalue_3 _returnvalue_4 _returnvalue_2 _returnvalue))
  ;[0 0 0] Find volume for snow ambience/weather and blizzard based on wind strength.
  (if (>= _returnvalue_6 2e+02)
    (Audio|Components|Audio|SetVolumeMultiplier (Variables|Default|GetBlizzard_Audio) (* (Math|Float|MapRangeClamped _returnvalue_6 2e+02 1.5e+03 0.5 1.0) _returnvalue_5) :!class /Script/Engine.AudioComponent)
    (return _returnvalue_5)
    (else
      (return _returnvalue_5))))